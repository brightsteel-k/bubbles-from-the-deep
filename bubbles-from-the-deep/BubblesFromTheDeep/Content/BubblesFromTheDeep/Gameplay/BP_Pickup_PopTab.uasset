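; BP_Pickup_PopTab is a pop tab pickup that the player collects by selecting it with the cursor.
; On BeginPlay, a drop timeline animates the skeletal mesh's relative height.
; The first selection notifies the Drowned game subsystem and sets a Collected flag to block repeat pickups.
; A collect timeline then moves the mesh vertically and spins it in yaw before the actor destroys itself.
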(event Custom|Collect
  (Class|DrownedGameSubsystem|CollectPopTab (Subsystems|GetDrownedGameSubsystem))
  (Variables|Default|SetbCollected true)
  (bind (_direction _relative_z_pos _relative_z_rot) (Timeline|Collect%20Animation PlayFromStart)
    (:Update
      (Transformation|SetRelativeLocationAndRotation (Variables|Default|GetSkeletalMesh) (Math|Vector|MakeVector 0.0 0.0 (* _relative_z_pos 4e+01)) (Math|Rotator|MakeRotator 0.0 0.0 _relative_z_rot) false false))
    (:Finished
      (Actor|DestroyActor))))

(event EventBeginPlay
  (bind _relative_z_pos (Timeline|Drop%20Animation PlayFromStart)
    (:Update
      (Transformation|SetRelativeLocation (Variables|Default|GetSkeletalMesh) (Math|Vector|MakeVector 0.0 0.0 (* _relative_z_pos 2e+01)) false false))))

(event EventOnCursorSelects
  (if (not (Variables|Default|GetbCollected))
    (CallFunction|Collect)))

(fn ConstructionScript)