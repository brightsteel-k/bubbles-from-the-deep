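; Game board slot that can hold a turret and shows cursor and click feedback through a material glow.
; BeginPlay creates a dynamic material instance on the mesh, and Tick eases its Glow parameter toward a target.
; Cursor select and deselect set the target on empty slots, and clearing a turret resets it.
; Valid and invalid clicks snap the current glow bright or off, which then eases back to the target.
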(event Custom|Tick%20Glow%20Param
  (params (Delta%20Seconds :type Float%20%28double-precision%29))
  ;[1 1 1] UI Responses
  (CallFunction|SetGlowParam (Math|Interpolation|FInterpTo (Variables|GlowAnimation|GetCurrent%20Glow%20Param) (Variables|GlowAnimation|GetTarget%20Glow%20Param) Delta%20Seconds 1e+01)))

(event Custom|On%20Invalid%20Click
  ;[1 1 1] UI Responses
  (CallFunction|SetGlowParam 0.0))

(event Custom|OnValid%20Click
  ;[1 1 1] UI Responses
  (CallFunction|SetGlowParam 2.0))

(event EventOnTurretPlaced
  ;[1 1 1] UI Responses
)

(event EventOnTurretCleared
  ;[1 1 1] UI Responses
  (|CallParentFunction)
  (Variables|GlowAnimation|SetTarget%20Glow%20Param 0.0))

(event EventOnCursorDeselects
  ;[1 1 1] UI Responses
  (if (not (Class|GameBoardSlot|HasTurret))
    (Variables|GlowAnimation|SetTarget%20Glow%20Param 0.0)))

(event EventBeginPlay
  (bind _mesh (Variables|Default|GetMesh))
  (bind _returnvalue (Rendering|Material|CreateDynamicMaterialInstance _mesh 0 (Rendering|Material|GetMaterial _mesh 0) "None" :!class /Script/Engine.PrimitiveComponent))
  (Variables|GameBoardSlot|SetSlot%20Material _returnvalue))

(event EventOnCursorSelects
  ;[1 1 1] UI Responses
  (if (not (Class|GameBoardSlot|HasTurret))
    (Variables|GlowAnimation|SetTarget%20Glow%20Param 0.5)))

(event EventTick
  (params (DeltaSeconds :type Float%20%28single-precision%29))
  (CallFunction|TickGlowParam DeltaSeconds))

(fn ConstructionScript)

(fn SetGlowParam
  (params (New%20Glow%20Param :type Float%20%28double-precision%29))
  (bind _output_get (Variables|GlowAnimation|SetCurrent%20Glow%20Param New%20Glow%20Param))
  (Rendering|Material|SetScalarParameterValue (Variables|GameBoardSlot|GetSlot%20Material) "Glow" _output_get :!class /Script/Engine.MaterialInstanceDynamic))