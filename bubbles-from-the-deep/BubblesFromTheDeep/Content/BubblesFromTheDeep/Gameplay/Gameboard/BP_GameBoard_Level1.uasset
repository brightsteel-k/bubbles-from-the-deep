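; BP_GameBoard_Level1 is the Level 1 game board, a child Blueprint that pre-populates its slots with coral turrets at BeginPlay.
; After the parent BeginPlay, it loops over GameBoardSlots, placing a TheWorld turret in the last slot and randomly placing TheFool turrets in roughly 40% of the others.
; This placement logic is marked as temporary, and the construction script only calls the parent.
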(event EventBeginPlay
  (bind _gameboardslots (Variables|Default|GetGameBoardSlots))
  (|CallParentFunction)
  ;[1 1 1] Temp
  (for (_array_element _array_index) _gameboardslots
    (if (== _array_index (- (Utilities|Array|Length _gameboardslots) 1))
      (Class|GameBoardSlot|PlaceTurret _array_element "/Game/BubblesFromTheDeep/Gameplay/CoralTurrets/BP_CoralTurret_TheWorld.BP_CoralTurret_TheWorld_C")
      (elif (> (Math|Random|RandomFloat) 0.6)
        (Class|GameBoardSlot|PlaceTurret _array_element "/Game/BubblesFromTheDeep/Gameplay/CoralTurrets/BP_CoralTurret_TheFool.BP_CoralTurret_TheFool_C")))))

(fn ConstructionScript
  (|CallParentFunction))