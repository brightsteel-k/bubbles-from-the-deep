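; Coral turret Blueprint for Bubbles From The Deep that smoothly turns toward a target rotation.
; AnimateRotateTo stores the target, and Tick eases the actor toward it with RInterpTo until nearly equal.
; CanTriggerAbility always returns false, while placement and tick events pass through to the parent class.
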(event EventTick
  (params (DeltaSeconds :type Float%20%28single-precision%29))
  (bind _returnvalue (Transformation|GetActorRotation))
  (|CallParentFunction DeltaSeconds)
  (if (not (Utilities|Operators|EqualEqual (Variables|Animations|GetTarget%20Rotation) _returnvalue 0.01))
    (Transformation|SetActorRotation (Math|Interpolation|RInterpTo _returnvalue (Variables|Animations|GetTarget%20Rotation) DeltaSeconds 1.0))))

(event EventOnTurretPlaced
  (params (Slot :type Game%20Board%20Slot%20Object%20Reference))
  (|CallParentFunction Slot))

(fn ConstructionScript)

(fn CanTriggerAbility
  (return false))

(fn AnimateRotateto
  (params (TargetRotation :type Rotator))
  (Variables|Animations|SetTarget%20Rotation TargetRotation))