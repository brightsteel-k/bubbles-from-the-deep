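; Turret ability component that gives a coral turret a single-target attack against monsters.
; On BeginPlay it caches the owning coral turret and its skeletal mesh.
; When triggered, it runs the parent ability, animates the turret's rotation toward the current target on the horizontal plane, and plays the attack montage.
; The montage's "Attack" notify applies the damage, syncing the hit with the animation.
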(event EventBeginPlay
  (bind _asbp_coral_turret (Utilities|Casting|CastToBP_CoralTurret (Variables|Default|GetCoralTurret)))
  (bind _output_get (Variables|SingleTargetAttack|SetBP%20Coral%20Turret _asbp_coral_turret))
  (Variables|SingleTargetAttack|SetTurret%20Mesh (Variables|/Game/BubblesFromTheDeep/Gameplay/CoralTurrets/BP_CoralTurret.BP_CoralTurret_C|GetSkeletalMesh _output_get)))

(event EventTick
  (params (DeltaSeconds :type Float%20%28single-precision%29)))

(event EventTriggerAbility
  (bind _currenttarget (Variables|Default|GetCurrentTarget))
  (bind _coralturret (Variables|Default|GetCoralTurret))
  (bind _returnvalue (Transformation|GetActorLocation _currenttarget))
  (bind _returnvalue_2 (Transformation|GetActorLocation _coralturret))
  (bind _returnvalue_3 (- _returnvalue _returnvalue_2))
  (|CallParentFunction)
  (Default|AnimateRotateto (Variables|SingleTargetAttack|GetBP%20Coral%20Turret) (Math|Rotator|MakeRotfromX (Math|Vector|MakeVector (.x _returnvalue_3) (.y _returnvalue_3) 0.0)))
  (bind _notifyname (Animation|Montage|PlayMontage (Variables|SingleTargetAttack|GetTurret%20Mesh) (Variables|SingleTargetAttack|GetAttack%20Animation))
    (:OnNotifyBegin
      (if (== _notifyname "Attack")
        (Class|DrossMonster|MonsterTakeDamage (Variables|Default|GetCurrentTarget) (Variables|SingleTargetAttack|GetDamage%20Amount))))))