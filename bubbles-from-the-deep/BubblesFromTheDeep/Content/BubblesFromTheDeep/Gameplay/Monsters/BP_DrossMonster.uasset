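; BP_DrossMonster is an enemy monster that attacks coral turrets, paired with its own AI controller.
; Entering advancing mode switches it to walking, enables blocking on a custom collision channel, lowers gravity and plays a timeline that offsets the mesh vertically.
; Capsule hits on turrets are reported to the controller, and attacks deal damage on the montage's Attack notify.
; Death runs the parent logic, then destroys the actor after a short delay.
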(event OnComponentHit(CapsuleComponent)
  (params (HitComponent :type Primitive%20Component%20Object%20Reference) (OtherActor :type Actor%20Object%20Reference) (OtherComp :type Primitive%20Component%20Object%20Reference) (NormalImpulse :type Vector :default "0, 0, 0") (Hit :type Hit%20Result%20Structure%20%28by%20ref%29))
  (bind _asbp_coral_turret (Utilities|Casting|CastToBP_CoralTurret OtherActor))
  (Default|OnEncounterTurret (Variables|DrossMonster|GetDross%20Monster%20Controller) _asbp_coral_turret))

(event EventBeginPlay
  (Variables|DrossMonster|SetMesh%20Relative%20Location (Variables|/Script/Engine.SceneComponent|GetRelativeLocation (Variables|Character|GetMesh)))
  (bind _asbp_aicdross_monster (Utilities|Casting|CastToBP_AICDrossMonster (Pawn|GetController)))
  (Variables|DrossMonster|SetDross%20Monster%20Controller _asbp_aicdross_monster))

(event EventEnterAdvancingMode
  (Pawn|Components|CharacterMovement|SetMovementMode (Variables|Character|GetCharacterMovement) "MOVE_Walking" 0)
  (Collision|SetCollisionResponsetoChannel (Variables|Default|GetCapsuleComponent) "ECC_GameTraceChannel1" "ECR_Block")
  (Variables|/Script/Engine.CharacterMovementComponent|SetGravityScale (Variables|Character|GetCharacterMovement) 0.5)
  (bind _relative_z_pos (Timeline|Rise%20to%20Advance%20Anim PlayFromStart)
    (:Update
      (Transformation|SetRelativeLocation (Variables|Character|GetMesh) (+ (Math|Vector|MakeVector 0.0 0.0 (* _relative_z_pos 1e+01)) (Variables|DrossMonster|GetMesh%20Relative%20Location)) true false))))

(event EventDie
  (|CallParentFunction)
  (Utilities|FlowControl|Delay 0.2)
  (Actor|DestroyActor))

(event EventAttackTurret
  (params (TargetTurret :type Coral%20Turret%20Object%20Reference))
  (bind _notifyname (Animation|Montage|PlayMontage (Variables|Character|GetMesh) (Variables|DrossMonster|GetAttack%20Montage))
    (:OnNotifyBegin
      (if (== _notifyname "Attack")
        (Class|CoralTurret|TurretTakeDamage TargetTurret (Variables|Default|GetAttackDamage))))))

(fn ConstructionScript)