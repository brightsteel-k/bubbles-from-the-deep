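; AI controller for the Dross monster, which rises upward, advances toward a destination slot and attacks turrets it encounters along the way.
; Tick runs a phase state machine that drives movement input for rising, advancing and chasing a turret.
; Within squared XY attack range, it stops and attacks on a self-rescheduling cooldown timer.
; When the target dies, it clears the timer and resumes advancing.
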(event Custom|Tick%20Rising%20State
  (params (Delta%20Seconds :type Float%20%28double-precision%29))
  (bind _destinationslot (Variables|Default|GetDestinationSlot))
  (bind _drossmonster (Variables|Default|GetDrossMonster))
  (bind _drossmonster_2 (Variables|Default|GetDrossMonster))
  (bind _returnvalue (Transformation|GetActorLocation _destinationslot))
  (bind _returnvalue_2 (Transformation|GetActorLocation _drossmonster))
  (bind _returnvalue_3 (- _returnvalue _returnvalue_2))
  (bind (_x _y _z) (Math|Vector|BreakVector _returnvalue_3))
  (Utilities|FlowControl|Sequence
    (:then_0
      (Pawn|Input|AddMovementInput _drossmonster_2 "0.000000,0.000000,1.000000" (Variables|RiseAnimation|GetRise%20Speed%20Multiplier) false)
      (Transformation|SetActorRotation _drossmonster_2 (Math|Rotator|MakeRotfromX (Math|Vector|MakeVector _x _y 0.0)) true))
    (:then_1
      (if (> (* _z -1.0) (Components|Capsule|GetScaledCapsuleHalfHeight (Variables|/Script/Engine.Character|GetCapsuleComponent _drossmonster)))
        (CallFunction|EndRisingPhase)))))

(event Custom|Trigger%20Recurring%20Attack
  (bind _drossmonster (Variables|Default|GetDrossMonster))
  (if (Variables|/Script/BubblesFromTheDeep.DrossMonster|GetbIsAlive _drossmonster)
    (Class|DrossMonster|AttackTurret _drossmonster (Variables|Default|GetCurrentTarget))
    (bind _returnvalue (Utilities|Time|SetTimerbyEvent (delegate Custom|Trigger%20Recurring%20Attack) (Variables|/Script/BubblesFromTheDeep.DrossMonster|GetAttackCooldown _drossmonster)))))

(event Custom|Stop%20Attacking
  (Utilities|Time|ClearandInvalidateTimerbyHandle (stale Custom|Trigger%20Recurring%20Attack _returnvalue)))

(event Custom|Start%20Attack%20Phase
  (AI|Navigation|StopMovement)
  (Variables|Default|SetBehaviorPhase "Attacking")
  (CallFunction|TriggerRecurringAttack))

(event Custom|Tick%20Aggro%20Phase
  (bind _currenttarget (Variables|Default|GetCurrentTarget))
  (bind _drossmonster (Variables|Default|GetDrossMonster))
  (bind _returnvalue (Transformation|GetActorLocation _currenttarget))
  (bind _returnvalue_2 (Transformation|GetActorLocation _drossmonster))
  (bind _returnvalue_3 (- _returnvalue _returnvalue_2))
  (if (> (Class|KismetMathLibrary|VSizeXYSquared _returnvalue_3) (Variables|AICDrossMonster|GetAttack%20Range%20Squared))
    (Pawn|Input|AddMovementInput (Variables|Default|GetDrossMonster) _returnvalue_3 1.0 false)
    (else
      (CallFunction|StartAttackPhase))))

(event Custom|Start%20Aggro%20Phase
  (params (Turret%20Target :type BP%20Coral%20Turret%20Object%20Reference))
  (Class|AICDrossMonster|SetCurrentTarget Turret%20Target)
  (Variables|Default|SetBehaviorPhase "Aggroing"))

(event Custom|On%20Encounter%20Turret
  (params (Turret :type BP%20Coral%20Turret%20Object%20Reference))
  (if (Variables|/Script/BubblesFromTheDeep.CoralTurret|GetbIsAlive Turret)
    (switch Utilities|FlowControl|Switch|SwitchonEMonsterBehaviorPhase (Variables|Default|GetBehaviorPhase)
      (:Advancing
        (CallFunction|StartAggroPhase Turret)))))

(event EventBeginPlay
  (|CallParentFunction))

(event EventTick
  (params (DeltaSeconds :type Float%20%28single-precision%29))
  (bind _drossmonster (Variables|Default|GetDrossMonster))
  (switch Utilities|FlowControl|Switch|SwitchonEMonsterBehaviorPhase (Variables|Default|GetBehaviorPhase)
    (:Rising
      (CallFunction|TickRisingState DeltaSeconds))
    (:Advancing
      (Pawn|Input|AddMovementInput _drossmonster (- (Transformation|GetActorLocation (Variables|Default|GetDestinationSlot)) (Transformation|GetActorLocation _drossmonster)) 1.0 false))
    (:Aggroing
      (CallFunction|TickAggroPhase))))

(event EventStart
  (|CallParentFunction)
  (Variables|AICDrossMonster|SetAttack%20Range%20Squared (Math|Float|Square (Variables|/Script/BubblesFromTheDeep.DrossMonster|GetAttackRange (Variables|Default|GetDrossMonster)))))

(event EventOnCurrentTargetDies
  (|CallParentFunction)
  (switch Utilities|FlowControl|Switch|SwitchonEMonsterBehaviorPhase (Variables|Default|GetBehaviorPhase)
    (:Aggroing
      _)
    (:Attacking
      _))
  (CallFunction|StopAttacking)
  (Variables|Default|SetBehaviorPhase "Advancing"))

(fn ConstructionScript)

(fn EndRisingPhase
  (Variables|Default|SetBehaviorPhase "Advancing")
  (Class|DrossMonster|EnterAdvancingMode (Variables|Default|GetDrossMonster)))