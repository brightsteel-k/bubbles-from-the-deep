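; Player pawn for Bubbles From The Deep with an orbit camera and hover-to-collect pickups.
; Q and E step a target yaw in opposite directions, repeating while held through delay-and-gate loops.
; Tick eases the PlayerPivot toward that yaw and line traces from the visible mouse cursor into the world.
; Any pop tab pickup the trace hits is collected immediately, with no click needed.
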(event Custom|Tick%20Orbit%20Controls
  (params (DeltaTime :type Float%20%28double-precision%29))
  ;[1 1 1] Orbit Camera Controls
  (bind _output_get (Variables|Orbit|SetCurrent%20Rotation (Math|Interpolation|FInterpTo (Variables|Orbit|GetCurrent%20Rotation) (Variables|Orbit|GetTarget%20Rotation) DeltaTime 1.0)))
  (Transformation|SetRelativeRotation (Variables|Default|GetPlayerPivot) (Math|Rotator|MakeRotator 0.0 0.0 _output_get) false false))

(event Custom|Check%20Cursor%20Select%20Objects
  (bind _returnvalue (Game|GetPlayerController 0))
  (bind (_worldlocation _worlddirection) (Game|Player|ConvertMouseLocationToWorldSpace _returnvalue))
  (bind (_outhit _returnvalue_2) (Collision|LineTraceByChannel _worldlocation (+ _worldlocation (* _worlddirection 1e+03)) "TraceTypeQuery3" false 0 "None" true "(R=1.000000,G=0.000000,B=0.000000,A=1.000000)" "(R=0.000000,G=1.000000,B=0.000000,A=1.000000)" 1.0))
  (if _returnvalue_2
    (CallFunction|OnCursorSelectsActor (.HitActor (Collision|BreakHitResult _outhit)))))

(event EventBeginPlay
  (Variables|/Script/Engine.PlayerController|SetbShowMouseCursor (Game|GetPlayerController 0) true))

(event EventTick
  (params (DeltaSeconds :type Float%20%28single-precision%29))
  (CallFunction|TickOrbitControls DeltaSeconds)
  (CallFunction|CheckCursorSelectObjects))

(event Input|KeyboardEvents|E
  (params (Key :type Key%20Structure :default "None"))
  ;[1 1 1] Orbit Camera Controls
  (:Pressed
    (Variables|Orbit|SetTarget%20Rotation (+ (Variables|Orbit|GetTarget%20Rotation) -1e+01) :!label _label)
    (Utilities|FlowControl|Sequence
      (:then_0
        (Utilities|FlowControl|RetriggerableDelay 0.4)
        (Utilities|FlowControl|Gate true :!label _label_2
          (:Exit
            (goto _label))))
      (:then_1
        (goto _label_2 Open))))
  (:Released
    (goto _label_2 Close)))

(event Input|KeyboardEvents|Q
  (params (Key :type Key%20Structure :default "None"))
  ;[1 1 1] Orbit Camera Controls
  (:Pressed
    (Variables|Orbit|SetTarget%20Rotation (+ (Variables|Orbit|GetTarget%20Rotation) 1e+01) :!label _label)
    (Utilities|FlowControl|Sequence
      (:then_0
        (Utilities|FlowControl|RetriggerableDelay 0.4)
        (Utilities|FlowControl|Gate true :!label _label_2
          (:Exit
            (goto _label))))
      (:then_1
        (goto _label_2 Open))))
  (:Released
    (goto _label_2 Close)))

(fn ConstructionScript)

(fn OnCursorSelectsActor
  (params (Actor :type Actor%20Object%20Reference))
  (bind _asbp_pickup_pop_tab (Utilities|Casting|CastToBP_Pickup_PopTab Actor))
  (Default|Collect _asbp_pickup_pop_tab))