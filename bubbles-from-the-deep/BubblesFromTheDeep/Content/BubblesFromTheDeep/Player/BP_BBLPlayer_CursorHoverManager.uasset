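; Player-side cursor manager that shows the mouse and handles hovering over and clicking objects on the game board.
; Every tick it line-traces from the deprojected mouse position and tracks the hit actor as CurrentSelection, sending select and deselect messages when it changes.
; Left-clicking a selected BP_GameBoardSlot without a turret triggers its valid-click response and places a hardcoded BP_CoralTurret_TheFool.
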(event Custom|Check%20Cursor%20Select%20Objects
  (bind _returnvalue (Game|GetPlayerController 0))
  (bind (_worldlocation _worlddirection) (Game|Player|ConvertMouseLocationToWorldSpace _returnvalue))
  (bind (_outhit _returnvalue_2) (Collision|LineTraceByChannel _worldlocation (+ _worldlocation (* _worlddirection 1e+03)) "TraceTypeQuery3" false 0 "None" true "(R=1.000000,G=0.000000,B=0.000000,A=1.000000)" "(R=0.000000,G=1.000000,B=0.000000,A=1.000000)" 1.0))
  (if _returnvalue_2
    (CallFunction|OnCursorHitsActor (.HitActor (Collision|BreakHitResult _outhit)))
    (else
      (CallFunction|OnCursorsHitsNoActor))))

(event EventTick
  (params (DeltaSeconds :type Float%20%28single-precision%29))
  (CallFunction|CheckCursorSelectObjects))

(event EventBeginPlay
  (Variables|/Script/Engine.PlayerController|SetbShowMouseCursor (Game|GetPlayerController 0) true))

(event Input|MouseEvents|LeftMouseButton
  (params (Key :type Key%20Structure :default "None"))
  (:Pressed
    (Utilities|FlowControl|Sequence
      (:then_0
        (bind _asbp_game_board_slot (Utilities|Casting|CastToBP_GameBoardSlot (Variables|Default|GetCurrent%20Selection)))
        (if (not (Class|GameBoardSlot|HasTurret _asbp_game_board_slot))
          (Default|OnValidClick _asbp_game_board_slot)
          (Class|GameBoardSlot|PlaceTurret _asbp_game_board_slot "/Game/BubblesFromTheDeep/Gameplay/CoralTurrets/BP_CoralTurret_TheFool.BP_CoralTurret_TheFool_C"))))))

(fn OnCursorHitsActor
  (params (Actor :type Actor%20Object%20Reference))
  (bind _current_selection (Variables|Default|GetCurrent%20Selection))
  (Utilities|IsValid _current_selection
    (:Is%20Valid
      (if (not (== Actor _current_selection))
        (CallFunction|DeselectOldActor)
        (CallFunction|SelectNewActor Actor :!label _label)))
    (:Is%20Not%20Valid
      (goto _label))))

(fn OnCursorsHitsNoActor
  (CallFunction|DeselectOldActor))

(fn SelectNewActor
  (params (Actor :type Actor%20Object%20Reference))
  (bind _output_get (Variables|Default|SetCurrent%20Selection Actor))
  (Class|BPICursorSelectionActor|OnCursorSelects(Message) _output_get))

(fn DeselectOldActor
  (Utilities|IsValid (Variables|Default|GetCurrent%20Selection)
    (:Is%20Valid
      (Class|BPICursorSelectionActor|OnCursorDeselects(Message) (Variables|Default|GetCurrent%20Selection))
      (Variables|Default|SetCurrent%20Selection 0))))